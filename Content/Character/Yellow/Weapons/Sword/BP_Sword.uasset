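; BP_Sword is a networked melee weapon that damages pawns caught in its hitbox.
; AttackWeapon enables collision on the server, and Tick calls ServerHitbox on any overlap, setting the RepNotify variable Attacking.
; OnRep_Attacking runs an authority-only hitbox query that excludes a player character derived from the attacker's index and returns after damaging the first pawn.
; A hit triggers FinishedAttack, which spawns an explosion with sound and disables collision.
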(event `Attack Weapon`
  (params (PlayerIndexLocal :type Integer))
  ;[1 1 1] Attack Input Function
  (set `self.PlayerIndexLocal` PlayerIndexLocal)
  (`/Engine/EditorBlueprintResources/ActorMacros.Switch Has Authority`
    (:`Authority`
      (`PrimitiveComponent.SetCollisionEnabled` "QueryAndPhysics"))))

(event `self.ReceiveBeginPlay`
  ;[1 1 1] Initialize Collision for Hitbox (off)
  (`self.InitCollisionHitbox`))

(event `self.ReceiveTick`
  (params (DeltaSeconds :type "Float (single-precision)"))
  ;[1 1 1] Custom Hitbox Event Trigger
  (if (!= (`KismetArrayLibrary.Array_Length` (`PrimitiveComponent.GetOverlappingActors` null)) 0)
    (`self.ServerHitbox`)))

(event `ServerHitbox`
  ;[1 1 1] Custom Hitbox Event Trigger
  (set `self.Attacking` true))

(event `FinishedAttack`
  ;[1 1 1] After Attack
  (bind _returnvalue (`GameplayStatics.SpawnEmitterAtLocation` "/Game/Particles/P_Explosion.P_Explosion" (`SceneComponent.GetSocketLocation` "None")))
  (`PrimitiveComponent.SetCollisionEnabled` "NoCollision")
  (`GameplayStatics.PlaySoundAttached` "/Game/StarterContent/Audio/Explosion01.Explosion01" _returnvalue))

(fn `ApplyAttacking`
  (returns (NumOverlapActors :type Integer))
  (`/Engine/EditorBlueprintResources/ActorMacros.Switch Has Authority`
    (:`Authority`
      (bind _outactors (`KismetSystemLibrary.ComponentOverlapActors_NEW` (`self.Hitbox`) (`SceneComponent.K2_GetComponentToWorld`) (`|MakeArray` "ObjectTypeQuery3" :!type "EngineTypes.EObjectTypeQuery Enum") null (`|MakeArray` (`GameplayStatics.GetPlayerCharacter` (- (`self.PlayerIndexLocal`) (`PlayerState.PlayerId` (`Controller.PlayerState` (`GameplayStatics.GetPlayerController` 0))))) :!type "Actor Object Reference")))
      (for _array_element _outactors
        (`GameplayStatics.ApplyDamage` _array_element (`self.SwordDamage`) (`self.GetInstigatorController`) self)
        (return (`KismetArrayLibrary.Array_Length` _outactors))))))

(fn `InitCollisionHitbox`
  (`PrimitiveComponent.SetCollisionEnabled` "NoCollision"))

(fn `OnRep_Attacking`
  (if (`self.Attacking`)
    (bind _numoverlapactors (`self.ApplyAttacking`))
    (if (!= _numoverlapactors 0)
      (`self.FinishedAttack`))))

(fn `UserConstructionScript`)