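; BP_Bomb is a bouncing bomb projectile that explodes and damages nearby Pawns once its bounce count reaches four.
; Each bounce sets Armed on the authority, and its RepNotify increments the count.
; On detonation, a server-only sphere overlap applies damage with instigator credit, while OnExplosion spawns particles and hides the actor before a short lifespan removes it.
; The count relies on the notify re-firing although Armed never resets.
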(event `self.ReceiveBeginPlay`)

(event `self.ReceiveActorBeginOverlap`
  (params (OtherActor :type "Actor Object Reference")))

(event `self.ReceiveTick`
  (params (DeltaSeconds :type "Float (single-precision)")))

(event `self.ProjectileMovement.OnProjectileBounce`
  (params (ImpactResult :type "EngineTypes.HitResult Structure (by ref)") (ImpactVelocity :type "Object.Vector Structure (by ref)"))
  (`/Engine/EditorBlueprintResources/ActorMacros.Switch Has Authority`
    (:`Authority`
      (set `self.Armed` true))))

(event `OnExplosion`
  (`GameplayStatics.SpawnEmitterAtLocation` (`self.ExplosionEffects`) (`self.K2_GetActorLocation`))
  (`self.SetActorEnableCollision` false)
  (`self.SetActorHiddenInGame` true))

(fn `ApplyExplosionDamage`
  (`/Engine/EditorBlueprintResources/ActorMacros.Switch Has Authority`
    (:`Authority`
      (bind _outactors (`KismetSystemLibrary.SphereOverlapActors_NEW` (`self.K2_GetActorLocation`) (`self.ExplosionRadius`) (`|MakeArray` "ObjectTypeQuery3" :!type "EngineTypes.EObjectTypeQuery Enum")))
      (for _array_element _outactors
        (`GameplayStatics.ApplyDamage` _array_element (`self.ExplosionDamage`) (`self.GetInstigatorController`) self)))))

(fn `OnRep_Armed`
  (if (`self.Armed`)
    (set `self.NumberBounce` (+ (`self.NumberBounce`) 1))
    (if (>= (`self.NumberBounce`) 4)
      (`self.ApplyExplosionDamage`)
      (`self.OnExplosion`)
      (`self.SetLifeSpan` 2.0))))

(fn `UserConstructionScript`)